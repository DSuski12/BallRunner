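; BP_restart restarts the current level when the first player's pawn leaves its Box volume.
; The Box end-overlap event fades the camera to black, waits for the fade to finish, then reopens the level by its current name.
; BeginPlay fades the camera in from white.
; Any other actor leaving the box only prints a debug string.
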(event OnComponentEndOverlap(Box)
  (params (OverlappedComponent :type Primitive%20Component%20Object%20Reference) (OtherActor :type Actor%20Object%20Reference) (OtherComp :type Primitive%20Component%20Object%20Reference) (OtherBodyIndex :type Integer))
  (if (== OtherActor (Game|Player|GetPlayerPawn 0))
    (CameraFades|StartCameraFade (Game|GetPlayerCameraManager 0) 0.0 1.0 2.0 "(R=0.000000,G=0.000000,B=0.000000,A=1.000000)" false false)
    (Utilities|FlowControl|Delay 2.0)
    (bind _returnvalue (Game|GetCurrentLevelName true))
    (Game|OpenLevel(byName) (Utilities|String|StringToName _returnvalue))
    (else
      (Development|PrintString "Hello"))))

(event EventBeginPlay
  (CameraFades|StartCameraFade (Game|GetPlayerCameraManager 0) 1.0 0.0 2.0 "(R=1.000000,G=1.000000,B=1.000000,A=1.000000)" false false))

(fn ConstructionScript)