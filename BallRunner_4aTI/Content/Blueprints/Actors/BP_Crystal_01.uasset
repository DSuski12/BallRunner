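; A collectible crystal actor that flies into the player and vanishes when something overlaps its sphere.
; On overlap it caches its location, scale and point light intensity, then plays the CrystalTransform timeline.
; Timeline tracks lerp it toward the player pawn's current position each update while shrinking it to zero and dimming its light.
; The actor destroys itself when the timeline finishes; the overlap does not check which actor triggered it.
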(event OnComponentBeginOverlap(Sphere)
  (params (OverlappedComponent :type Primitive%20Component%20Object%20Reference) (OtherActor :type Actor%20Object%20Reference) (OtherComp :type Primitive%20Component%20Object%20Reference) (OtherBodyIndex :type Integer) (bFromSweep :type Boolean) (SweepResult :type Hit%20Result%20Structure%20%28by%20ref%29))
  (CallFunction|SetVariables)
  (bind (_direction _crystal_location _crystal_scale _crystal_light) (Timeline|CrystalTransform Play)
    (:Update
      (CallFunction|CrystalLocation _crystal_location)
      (CallFunction|CrystalScale _crystal_scale)
      (CallFunction|CrystalLight _crystal_light))
    (:Finished
      (Actor|DestroyActor))))

(fn ConstructionScript)

(fn CrystalLocation
  (params (Alpha :type Float%20%28single-precision%29))
  (Transformation|SetActorLocation (Math|Vector|Lerp(Vector) (Variables|Default|GetCrystal%20location) (Transformation|GetActorLocation (Game|Player|GetPlayerPawn 0)) Alpha) false false))

(fn CrystalScale
  (params (Alpha :type Float%20%28single-precision%29))
  (Transformation|SetActorScale3D (Math|Vector|Lerp(Vector) (Variables|Default|GetCrystal%20scale) "0, 0, 0" Alpha)))

(fn CrystalLight
  (params (Alpha :type Float%20%28single-precision%29))
  (Rendering|Components|Light|SetIntensity (Variables|Default|GetPointLight) (Math|Float|Lerp (Variables|Default|GetCrystal%20intensity) 0.0 Alpha)))

(fn SetVariables
  (Variables|Default|SetCrystal%20scale (Transformation|GetActorScale3D))
  (Variables|Default|SetCrystal%20location (Transformation|GetActorLocation))
  (Variables|Default|SetCrystal%20intensity (Variables|/Script/Engine.LightComponentBase|GetIntensity (Variables|Default|GetPointLight))))